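; BP_VectorWarShip is the visual actor for one player's ship in VectorWar.
; On BeginPlay it creates a dynamic material on its cone mesh and picks the color from PlayerIndex.
; Each Tick it snaps the root, without sweep, to the transform returned by ShipTransform for that player, computing no movement in its own graph.
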(event `self.ReceiveBeginPlay`
  (bind _returnvalue (`PrimitiveComponent.CreateDynamicMaterialInstance` (`self.Cone`) 0 "/Game/Materials/M_ShipMaterial.M_ShipMaterial" "None"))
  (bind _output_get (set `self.ShipMaterial` _returnvalue))
  (`MaterialInstanceDynamic.SetVectorParameterValue` _output_get "Color" (select `int` (`self.PlayerIndex`) :`0` (make `LinearColor` 1.0 0.0 0.0 1.0) :`1` (make `LinearColor` 0.0 1.0 0.0 1.0) :`2` (make `LinearColor` 0.0 0.0 1.0 1.0) :`3` (make `LinearColor` 0.5 0.5 0.5 1.0))))

(event `self.ReceiveTick`
  (params (DeltaSeconds :type "Float (single-precision)"))
  (`SceneComponent.K2_SetWorldTransform` (`self.Root`) (`GameStateInterface.ShipTransform` (`self.PlayerIndex`)) false false))

(fn `UserConstructionScript`)